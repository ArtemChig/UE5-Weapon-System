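; Master bullet projectile actor that flies by physics and leaves surface-specific impact effects where it hits.
; On BeginPlay it configures its light, launches the Bullet component along actor forward and creates a decal material instance with a random hole variant.
; On hit it picks a Niagara system by physical surface type, spawns it along the hit normal, places a randomly sized decal facing the bullet-to-impact direction, then destroys itself.
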(event OnComponentHit(Bullet)
  (params (HitComponent :type Primitive%20Component%20Object%20Reference) (OtherActor :type Actor%20Object%20Reference) (OtherComp :type Primitive%20Component%20Object%20Reference) (NormalImpulse :type Vector :default "0, 0, 0") (Hit :type Hit%20Result%20Structure%20%28by%20ref%29))
  (bind (_bblockinghit _binitialoverlap _time _distance _location _impactpoint _normal _impactnormal _physmat) (Collision|BreakHitResult Hit))
  (bind _decal_size (Variables|Default|GetDecal_size))
  (bind (_x _y) (Math|Vector2D|BreakVector2D _decal_size))
  (Variables|Default|SetHit_location _location)
  (Variables|Default|SetHit_facing_rotation (Math|Rotator|MakeRotationfromAxes (Math|Vector|GetUnitDirection(Vector) (Transformation|GetWorldLocation (Variables|Default|GetBullet)) (Variables|Default|GetHit_location)) "0, 0, 0" "0, 0, 0"))
  (Variables|Default|SetHit_normal (Math|Rotator|MakeRotationfromAxes _normal "0, 0, 0" "0, 0, 0"))
  (Variables|Default|SetHit_system (Utilities|Select :Index (Variables|/Script/PhysicsCore.PhysicalMaterial|GetSurfaceType _physmat) :SurfaceType_Default 0 :SurfaceType1 "/Game/VFX/Weapon_system/Impacts/NS_Wood_impact.NS_Wood_impact" :SurfaceType2 "/Game/VFX/Weapon_system/Impacts/NS_Metal_impact.NS_Metal_impact" :SurfaceType3 "/Game/VFX/Weapon_system/Impacts/NS_Brick_impact.NS_Brick_impact" :SurfaceType4 "/Game/VFX/Weapon_system/Impacts/NS_Dirt_impact.NS_Dirt_impact" :SurfaceType5 "/Game/VFX/Weapon_system/Impacts/NS_Asphalt_impact.NS_Asphalt_impact" :SurfaceType6 "/Game/VFX/Weapon_system/Impacts/NS_Dirt_impact.NS_Dirt_impact" :SurfaceType7 "/Game/VFX/Weapon_system/Impacts/NS_Gravel_Impact.NS_Gravel_Impact"))
  (Rendering|Decal|SpawnDecalatLocation (Variables|Default|GetDecal_DMI) (Math|Conversions|ToVector(Float) (Math|Random|RandomFloatinRange _x _y)) (Variables|Default|GetHit_location) (Variables|Default|GetHit_facing_rotation) 5e+01)
  (Niagara|SpawnSystematLocation (Variables|Default|GetHit_system) (Variables|Default|GetHit_location) (Variables|Default|GetHit_normal))
  (Actor|DestroyActor self))

(event EventBeginPlay
  (Rendering|Components|Light|SetIntensity (Variables|Default|GetBullet_light) (Variables|Default|GetBullet_Light_intensity))
  (Rendering|Lighting|SetAttenuationRadius (Variables|Default|GetBullet_light) (Variables|Default|GetBullet_Light_Radius))
  (Physics|SetPhysicsLinearVelocity (Variables|Default|GetBullet) (* (Variables|Default|GetBullet_speed) (Math|Vector|GetForwardVector (Transformation|GetActorRotation))) false "None")
  (bind _returnvalue (Rendering|Material|CreateDynamicMaterialInstance "/Game/VFX/Weapon_system/Bullet/Materials/M_bullet_hole_decal.M_bullet_hole_decal" "None" "None" :!class /Script/Engine.KismetMaterialLibrary))
  (Variables|Default|SetDecal_DMI _returnvalue)
  (Rendering|Material|SetScalarParameterValue (Variables|Default|GetDecal_DMI) "hole_index" (Math|Conversions|ToFloat(Integer) (Math|Random|RandomIntegerinRange 0 2)) :!class /Script/Engine.MaterialInstanceDynamic))

(fn ConstructionScript)