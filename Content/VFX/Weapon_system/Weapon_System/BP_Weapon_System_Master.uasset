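; Master weapon actor for a VFX weapon system that fires a configurable bullet with a muzzle flash.
; The Shoot event spawns the BulletType actor at the weapon's transform, then passes it speed, light and decal size settings through SetVariables.
; It also spawns a scaled Niagara muzzle flash at the same location and rotation.
; Nothing in this Blueprint calls Shoot, and BeginPlay and the construction script are empty.
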(event Custom|Shoot
  (bind _returnvalue (Game|SpawnActorfromClass (Variables|Default|GetBullet%20Type) (Transformation|GetActorTransform) "Undefined" "MultiplyWithRoot" 0 0))
  (Default|SetVariables _returnvalue (Variables|Default|GetBullet%20Speed) (Variables|Default|GetBullet%20Light%20Radius) (Variables|Default|GetBullet%20Light%20Intensity) (Variables|Default|GetDecal%20Size))
  (Niagara|SpawnSystematLocation (Variables|Default|GetMuzzle_Flash_System) (Transformation|GetActorLocation) (Transformation|GetActorRotation) (Math|Conversions|ToVector(Float) (Variables|Default|GetMuzzle_Flash_scale))))

(event EventBeginPlay)

(fn ConstructionScript)