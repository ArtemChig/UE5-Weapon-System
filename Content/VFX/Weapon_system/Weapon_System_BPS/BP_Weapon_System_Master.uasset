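; Master weapon actor that fires a projectile with a muzzle flash effect when its Shoot event is called.
; Shoot spawns the BulletType actor at the weapon's transform, then a Niagara MuzzleFlashSystem at its location, sized by MuzzleFlashScale.
; The flash rotation treats the actor's roll, pitch and yaw as an X-axis direction vector rather than using the actor rotation directly.
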(event Custom|Shoot
  (bind _returnvalue (Transformation|GetActorRotation))
  (bind (_roll _pitch _yaw) (Math|Rotator|BreakRotator _returnvalue))
  (Game|SpawnActorfromClass (Variables|Default|GetBullet_type) (Transformation|GetActorTransform) "Undefined" "MultiplyWithRoot" 0 0)
  (Niagara|SpawnSystematLocation (Variables|Default|GetMuzzle_Flash_System) (Transformation|GetActorLocation) (Math|Conversions|RotationFromXVector (Math|Vector|MakeVector _roll _pitch _yaw)) (Math|Conversions|ToVector(Float) (Variables|Default|GetMuzzle_Flash_scale))))

(event EventBeginPlay)

(fn ConstructionScript)